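; Wand item Blueprint that grants the third-person character the Blink spell.
; A box overlap shows a text render while the character is inside and hides it on exit.
; SpellInteract runs once through a DoOnce, adding an ItemPickup widget to the viewport and setting BlinkSpell on the overlapping character.
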(event `self.Box.OnComponentBeginOverlap`
  (params (OverlappedComponent :type "PrimitiveComponent Object Reference") (OtherActor :type "Actor Object Reference") (OtherComp :type "PrimitiveComponent Object Reference") (OtherBodyIndex :type Integer) (bFromSweep :type Boolean) (SweepResult :type "HitResult Structure (by ref)"))
  (cast `/Game/ThirdPersonBP/Blueprints/ThirdPersonCharacter` OtherActor)
  (`SceneComponent.SetHiddenInGame` (`self.Text Render`) false false))

(event `self.Box.OnComponentEndOverlap`
  (params (OverlappedComponent :type "PrimitiveComponent Object Reference") (OtherActor :type "Actor Object Reference") (OtherComp :type "PrimitiveComponent Object Reference") (OtherBodyIndex :type Integer))
  (cast `/Game/ThirdPersonBP/Blueprints/ThirdPersonCharacter` OtherActor)
  (`SceneComponent.SetHiddenInGame` (`self.Text Render`) true false))

(event `/Game/ThirdPersonBP/Spells/SpellInteract.SpellInteract`
  (`/Engine/EditorBlueprintResources/StandardMacros.DoOnce` false
    (:`Completed`
      (bind _returnvalue (`|CreateWidget` "/Game/Items/ItemPickup.ItemPickup_C"))
      (bind _output_get (set `self.ItemRef` _returnvalue))
      (`UserWidget.AddToViewport` _output_get 0)
      (bind _asthird_person_character (cast `/Game/ThirdPersonBP/Blueprints/ThirdPersonCharacter` (stale `self.Box.OnComponentEndOverlap` OtherActor)))
      (set `/Game/ThirdPersonBP/Blueprints/ThirdPersonCharacter.Blink Spell` true _asthird_person_character))))

(fn `UserConstructionScript`)