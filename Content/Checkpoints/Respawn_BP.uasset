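; Checkpoint actor that saves a respawn point when the ThirdPersonCharacter overlaps its Box trigger.
; The overlap writes the character's current transform to SpawnTransform on the ThirdPersonGameMode, then sets the character's Mana to 1.0.
; It plays the checkpoint sound at the actor's location on every such overlap, as PlayCheckPointSound is set true just before it is tested.
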(event `self.Box.OnComponentBeginOverlap`
  (params (OverlappedComponent :type "PrimitiveComponent Object Reference") (OtherActor :type "Actor Object Reference") (OtherComp :type "PrimitiveComponent Object Reference") (OtherBodyIndex :type Integer) (bFromSweep :type Boolean) (SweepResult :type "HitResult Structure (by ref)"))
  (bind _asthird_person_character (cast `/Game/ThirdPersonBP/Blueprints/ThirdPersonCharacter` OtherActor))
  (bind _asthird_person_game_mode (cast `/Game/ThirdPersonBP/Blueprints/ThirdPersonGameMode` (`GameplayStatics.GetGameMode`)))
  (set `/Game/ThirdPersonBP/Blueprints/ThirdPersonGameMode.Spawn transform` (`self.GetTransform` _asthird_person_character) _asthird_person_game_mode)
  (bind _asthird_person_character_2 (cast `/Game/ThirdPersonBP/Blueprints/ThirdPersonCharacter` OtherActor))
  (set `/Game/ThirdPersonBP/Blueprints/ThirdPersonCharacter.Mana` 1.0 _asthird_person_character_2)
  (set `self.PlayCheckPointSound` true)
  (if (`self.PlayCheckPointSound`)
    (`GameplayStatics.PlaySoundAtLocation` "/Game/Checkpoints/Checkpointsound.Checkpointsound" (`self.K2_GetActorLocation`) (struct) 0.5 1.0 0.0 null null null)))

(fn `UserConstructionScript`)